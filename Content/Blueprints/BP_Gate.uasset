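; BP_Gate is a force field gate that opens for a player character carrying the matching keys.
; BeginPlay creates a dynamic forcefield material tinted by GateColour.
; When a BP_ThirdPersonCharacter enters the interaction zone, its KeysCollected tags are tested against the GateType tag query.
; A match immediately disables the field's collision, then a timeline animates the material's Opacity.
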(event `self.ReceiveBeginPlay`
  (bind _returnvalue (`PrimitiveComponent.CreateDynamicMaterialInstance` (`self.ForceField`) 0 "/Game/TeachersMarketplace/Assets/Architecture/Gate/Material/MI_forcefield.MI_forcefield" "None"))
  (set `self.ForcefieldDynMatRef` _returnvalue)
  (`MaterialInstanceDynamic.SetVectorParameterValue` (`self.ForcefieldDynMatRef`) "ColorMultiplier" (`self.GateColour`)))

(event `self.GateInteractionZone.OnComponentBeginOverlap`
  (params (OverlappedComponent :type "PrimitiveComponent Object Reference") (OtherActor :type "Actor Object Reference") (OtherComp :type "PrimitiveComponent Object Reference") (OtherBodyIndex :type Integer) (bFromSweep :type Boolean) (SweepResult :type "HitResult Structure (by ref)"))
  (bind _asbp_third_person_character (cast `/Game/ThirdPerson/Blueprints/BP_ThirdPersonCharacter` OtherActor))
  (if (`BlueprintGameplayTagLibrary.DoesContainerMatchTagQuery` (`/Game/ThirdPerson/Blueprints/BP_ThirdPersonCharacter.KeysCollected` _asbp_third_person_character) (`self.GateType`))
    (`self.OpenTheGate`)))

(event `OpenTheGate`
  (`PrimitiveComponent.SetCollisionEnabled` (`self.ForceField`) "NoCollision")
  (bind (_direction _opacity) (`Timeline|T_OpeningTheGate`)
    (:`Update`
      (`MaterialInstanceDynamic.SetScalarParameterValue` (`self.ForcefieldDynMatRef`) "Opacity" _opacity))))

(fn `UserConstructionScript`)